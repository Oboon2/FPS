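; Player character Blueprint that displays health on two widget components and removes the actor after its HP runs out.
; Each Tick casts both widgets to HPBarWidget and sets their Percent from CurrentHP over MaxHP, polling rather than using events.
; Tick also checks for exactly zero CurrentHP, then destroys the actor after a short delay.
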(event `self.ReceiveTick`
  (params (DeltaSeconds :type "Float (single-precision)"))
  (`|ExecutionSequence`
    (:`then_0`
      (`|ExecutionSequence`
        (:`then_0`
          (bind _ashpbar_widget (cast `/Game/Blueprints/UI/HPBarWidget` (`WidgetComponent.GetUserWidgetObject` (`self.Widget`))))
          (set `/Game/Blueprints/UI/HPBarWidget.Percent` (/ (`self.CurrentHP`) (`self.MaxHP`)) _ashpbar_widget))
        (:`then_1`
          (bind _ashpbar_widget_2 (cast `/Game/Blueprints/UI/HPBarWidget` (`WidgetComponent.GetUserWidgetObject` (`self.WidgetB`))))
          (set `/Game/Blueprints/UI/HPBarWidget.Percent` (/ (`self.CurrentHP`) (`self.MaxHP`)) _ashpbar_widget_2))))
    (:`then_1`
      (if (== (`self.CurrentHP`) 0.0)
        (`KismetSystemLibrary.Delay` 3.0)
        (`self.K2_DestroyActor`)))))

(fn `UserConstructionScript`)