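; BP_GM is a game manager that drives stage progression from StartStage through Stage01–03 to FinishStage.
; Every Tick it checks the current level name and counts Zombie-tagged actors, loading the next stage when none remain.
; StartStage and FinishStage use tagged actors as menu choices: clearing Zombies starts Stage01, clearing Enemy_Player actors quits.
; It also polls BP_MyCharacter's HP, opening FinishStage when it equals zero.
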(event `self.ReceiveTick`
  (params (DeltaSeconds :type "Float (single-precision)"))
  (bind _returnvalue (`GameplayStatics.GetCurrentLevelName` true))
  (set `self.CurrentLevel` _returnvalue)
  (`|ExecutionSequence`
    (:`then_0`
      (if (`KismetStringLibrary.EqualEqual_StrStr` (`self.CurrentLevel`) "StartStage")
        (`|ExecutionSequence`
          (:`then_0`
            (bind _outactors (`GameplayStatics.GetAllActorsWithTag` "Zombie"))
            (bind _output_get (set `self.Zombie` _outactors))
            (bind _output_get_2 (set `self.EnemyCount` (`KismetArrayLibrary.Array_Length` _output_get)))
            (if (== _output_get_2 0)
              (`KismetSystemLibrary.PrintString` "GameStart!")
              (`GameplayStatics.OpenLevel` "Stage01")))
          (:`then_1`
            (bind _outactors_2 (`GameplayStatics.GetAllActorsWithTag` "Enemy_Player"))
            (bind _output_get_3 (set `self.NewVar_0` _outactors_2))
            (bind _output_get_4 (set `self.EnemyPlayerCount` (`KismetArrayLibrary.Array_Length` _output_get_3)))
            (if (== _output_get_4 0)
              (`KismetSystemLibrary.PrintString` "Quit")
              (`KismetSystemLibrary.QuitGame` null "Quit"))))))
    (:`then_1`
      (if (`KismetStringLibrary.EqualEqual_StrStr` (`self.CurrentLevel`) "Stage01")
        (bind _outactors_3 (`GameplayStatics.GetAllActorsWithTag` "Zombie"))
        (bind _output_get_5 (set `self.Zombie` _outactors_3))
        (bind _output_get_6 (set `self.EnemyCount` (`KismetArrayLibrary.Array_Length` _output_get_5)))
        (if (== _output_get_6 0)
          (`KismetSystemLibrary.PrintString` "Stage01 Clear!!")
          (`GameplayStatics.OpenLevel` "Stage02"))))
    (:`then_2`
      (if (`KismetStringLibrary.EqualEqual_StrStr` (`self.CurrentLevel`) "Stage02")
        (bind _outactors_4 (`GameplayStatics.GetAllActorsWithTag` "Zombie"))
        (bind _output_get_7 (set `self.Zombie` _outactors_4))
        (bind _output_get_8 (set `self.EnemyCount` (`KismetArrayLibrary.Array_Length` _output_get_7)))
        (if (== _output_get_8 0)
          (`KismetSystemLibrary.PrintString` "Stage02 Clear!!")
          (`GameplayStatics.OpenLevel` "Stage03"))))
    (:`then_3`
      (if (`KismetStringLibrary.EqualEqual_StrStr` (`self.CurrentLevel`) "Stage03")
        (bind _outactors_5 (`GameplayStatics.GetAllActorsWithTag` "Zombie"))
        (bind _output_get_9 (set `self.Zombie` _outactors_5))
        (bind _output_get_10 (set `self.EnemyCount` (`KismetArrayLibrary.Array_Length` _output_get_9)))
        (if (== _output_get_10 0)
          (`KismetSystemLibrary.PrintString` "All Stage Clear!!")
          (`KismetSystemLibrary.PrintString` "All Stage Clear!!")
          (`GameplayStatics.OpenLevel` "FinishStage"))))
    (:`then_4`
      (if (`KismetStringLibrary.EqualEqual_StrStr` (`self.CurrentLevel`) "FinishStage")
        (`|ExecutionSequence`
          (:`then_0`
            (bind _outactors_6 (`GameplayStatics.GetAllActorsWithTag` "Zombie"))
            (bind _output_get_11 (set `self.Zombie` _outactors_6))
            (bind _output_get_12 (set `self.EnemyCount` (`KismetArrayLibrary.Array_Length` _output_get_11)))
            (if (== _output_get_12 0)
              (`KismetSystemLibrary.PrintString` "GameStart!")
              (`GameplayStatics.OpenLevel` "Stage01")))
          (:`then_1`
            (bind _outactors_7 (`GameplayStatics.GetAllActorsWithTag` "Enemy_Player"))
            (bind _output_get_13 (set `self.NewVar_0` _outactors_7))
            (bind _output_get_14 (set `self.EnemyPlayerCount` (`KismetArrayLibrary.Array_Length` _output_get_13)))
            (if (== _output_get_14 0)
              (`KismetSystemLibrary.PrintString` "Quit")
              (`KismetSystemLibrary.QuitGame` null "Quit"))))))
    (:`then_5`
      (bind _asbp_my_character (cast `/Game/Blueprints/Player/BP_MyCharacter` (`GameplayStatics.GetPlayerCharacter` 0)))
      (if (== (`MyCharacter.CurrentHP` _asbp_my_character) 0.0)
        (`KismetSystemLibrary.PrintString` "당신은 죽었습니다!!")
        (`KismetSystemLibrary.PrintString` "당신은 죽었습니다!!")
        (`GameplayStatics.OpenLevel` "FinishStage")))))

(fn `UserConstructionScript`)